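; Game instance that manages front-end menus and multiplayer sessions across levels.
; A save check opens the main menu, or the options menu with a welcome message when no save exists; most widgets are cached for reuse.
; Hosting and joining show a loading screen around session calls, with successful hosting opening the Lobby level.
; Session, network and travel failures route to an error display, whose body and string converters are empty stubs.
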(event `SaveGameCheck`
  (bind _returnvalue (`GameplayStatics.DoesSaveGameExist` (`self.PlayerSettingsSave`)))
  (if _returnvalue
    (`self.DisplayMainMenu`)
    (set `self.CreatedSaveFile` true)
    (else
      (`self.DisplayOptionsMenu`)
      (set `PlayerController.bShowMouseCursor` true (`GameplayStatics.GetPlayerController` 0)))))

(event `DisplayMainMenu`
  (bind _returnvalue (`GameplayStatics.GetPlayerController` 0))
  ;[1 1 1] Comment
  (`/Engine/EditorBlueprintResources/StandardMacros.IsValid` (`self.MainMenuUMG`)
    (:`Is Valid`
      _)
    (:`Is Not Valid`
      (bind _returnvalue_2 (`|CreateWidget` "/Game/UI/MainMenu/MainMenu.MainMenu_C" _returnvalue))
      (set `self.MainMenuUMG` _returnvalue_2)))
  (`UserWidget.AddToViewport` (`self.MainMenuUMG`) 0)
  (set `PlayerController.bShowMouseCursor` true _returnvalue))

(event `DisplayHostMenu`
  ;[1 1 1] Comment
  (`/Engine/EditorBlueprintResources/StandardMacros.IsValid` (`self.HostMenuUMG`)
    (:`Is Valid`
      _)
    (:`Is Not Valid`
      (bind _returnvalue (`|CreateWidget` "/Game/UI/MainMenu/HostMenu.HostMenu_C" (`GameplayStatics.GetPlayerController` 0)))
      (set `self.HostMenuUMG` _returnvalue)))
  (`UserWidget.AddToViewport` (`self.HostMenuUMG`) 0))

(event `DisplayServerMenu`
  ;[1 1 1] Comment
  (bind _returnvalue (`|CreateWidget` "/Game/UI/MainMenu/ServerMenu.ServerMenu_C" (`GameplayStatics.GetPlayerController` 0)))
  (`UserWidget.AddToViewport` _returnvalue 0))

(event `DisplayOptionsMenu`
  ;[1 1 1] Comment
  (`/Engine/EditorBlueprintResources/StandardMacros.IsValid` (`self.OptionsMenuUMG`)
    (:`Is Valid`
      _)
    (:`Is Not Valid`
      (bind _returnvalue (`|CreateWidget` "/Game/UI/MainMenu/OptionsMenu.OptionsMenu_C" (`GameplayStatics.GetPlayerController` 0)))
      (set `self.OptionsMenuUMG` _returnvalue)))
  (`UserWidget.AddToViewport` (`self.OptionsMenuUMG`) 0)
  (if (not (`self.CreatedSaveFile`))
    (set `/Game/UI/MainMenu/OptionsMenu.WelcomeMessageVis` "Visible" (`self.OptionsMenuUMG`))))

(event `LaunchLobby`
  (params (`N°OfPlayers` :type Integer) (LANEnabled :type Boolean) (ServerName :type Text))
  ;[1 1 1] Comment
  (set `self.MaxPlayers` `N°OfPlayers`)
  (set `self.ServerName` ServerName)
  (`self.DisplayLoadingScreen`)
  (`CreateSessionCallbackProxy.CreateSession` (`GameplayStatics.GetPlayerController` 0) (`self.MaxPlayers`) LANEnabled
    (:`OnSuccess`
      (`GameplayStatics.OpenLevel` "Lobby" true "listen"))
    (:`OnFailure`
      (`self.DisplayErrorMsg` "Failed to Create Session"))))

(event `DisplayLoadingScreen`
  ;[1 1 1] Comment
  (`/Engine/EditorBlueprintResources/StandardMacros.IsValid` (`self.LoadingScreenUMG`)
    (:`Is Valid`
      _)
    (:`Is Not Valid`
      (bind _returnvalue (`|CreateWidget` "/Game/UI/AllLevels/LoadingScreen.LoadingScreen_C" (`GameplayStatics.GetPlayerController` 0)))
      (set `self.LoadingScreenUMG` _returnvalue)))
  (`UserWidget.AddToViewport` (`self.LoadingScreenUMG`) 0))

(event `JoinServer`
  (params (SessionToJoin :type "BlueprintSessionResult Structure"))
  ;[1 1 1] Comment
  (`self.DisplayLoadingScreen`)
  (`JoinSessionCallbackProxy.JoinSession` (`GameplayStatics.GetPlayerController` 0) SessionToJoin
    (:`OnFailure`
      (`self.DisplayErrorMsg` "Failed To Join Session"))))

(event `self.HandleNetworkError`
  (params (FailureType :type "ENetworkFailure Enum" :default "NetDriverAlreadyExists") (bIsServer :type Boolean))
  ;[1 1 1] Comment
  (`self.DisplayErrorMsg` (`self.NetErrorToString` FailureType)))

(event `self.HandleTravelError`
  (params (FailureType :type "ETravelFailure Enum" :default "NoLevel"))
  ;[1 1 1] Comment
  (`self.DisplayErrorMsg` (`self.TravelErrorToString` FailureType)))

(event `DestroySessionCaller`
  (params (PC :type "PlayerController Object Reference"))
  ;[1 1 1] Comment
  (`DestroySessionCallbackProxy.DestroySession` PC))

(fn `NetErrorToString`
  (params (FailureType :type "ENetworkFailure Enum" :default "NetDriverAlreadyExists"))
  (returns (outString :type String))
  (return ""))

(fn `TravelErrorToString`
  (params (TravelErrorType :type "ETravelFailure Enum" :default "NoLevel"))
  (returns (OutString :type String))
  (return ""))